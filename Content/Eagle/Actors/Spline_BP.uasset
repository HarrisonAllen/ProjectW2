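; Spline actor that traces both eagle wings with particle system components that follow the animated wing mesh.
; BeginPlay reads numbered wing sockets on the Eagle_Mesh_Blueprint_Wing actor, builds left and right splines, and spawns a particle component per point.
; Tick re-reads the sockets, moves the spline points, then snaps particles to them, with both wings sharing one particle array.
; A disconnected graph maps third-person character arm rotations to wing rotations.
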(event EventBeginPlay
  (bind _r_socketpositions (Variables|Default|GetR_SocketPositions))
  (bind _l_socketpositions (Variables|Default|GetL_SocketPositions))
  (Spline|ClearSplinePoints (Variables|Default|GetLeftWingSpline) true)
  (Spline|ClearSplinePoints (Variables|Default|GetRightWingSpline) true)
  (Utilities|Array|Clear (Variables|Default|GetSpawnedParticles))
  (Utilities|FlowControl|Sequence
    (:then_0
      (bind _outactors (Actor|GetAllActorsOfClass "/Game/Eagle/Actors/Eagle_Mesh_Blueprint_Wing.Eagle_Mesh_Blueprint_Wing_C")) ; Begin Left Wing Spline and Particle Generation
      (Utilities|Array|Clear (Variables|Default|GetL_SocketPositions))
      (Utilities|Array|Add (Variables|Default|GetL_SocketPositions) (Transformation|GetSocketLocation (Variables|/Script/Engine.SkeletalMeshActor|GetSkeletalMeshComponent (Utilities|Array|Get(acopy) _outactors)) "LeftWingBase"))
      (for _index (range 1 15)
        (bind _output_get (Variables|Default|SetWingName (Utilities|String|BuildString(Integer) "" "LeftWing" _index)))
        (Utilities|Array|Add (Variables|Default|GetL_SocketPositions) (Transformation|GetSocketLocation (Variables|/Script/Engine.SkeletalMeshActor|GetSkeletalMeshComponent (Utilities|Array|Get(acopy) _outactors)) (Utilities|String|StringToName _output_get))))
      (Spline|SetSplinePoints (Variables|Default|GetLeftWingSpline) _l_socketpositions "World" true)
      (for _array_element _l_socketpositions
        (bind _returnvalue (AddComponent|AddParticleSystemComponent true (Math|Conversions|ToTransform(Vector) _array_element)))
        (Utilities|Array|Add (Variables|Default|GetSpawnedParticles) _returnvalue)))
    (:then_1
      (bind _outactors_2 (Actor|GetAllActorsOfClass "/Game/Eagle/Actors/Eagle_Mesh_Blueprint_Wing.Eagle_Mesh_Blueprint_Wing_C")) ; Begin Right Wing Spline and Particle Generation
      (Utilities|Array|Clear (Variables|Default|GetR_SocketPositions))
      (Utilities|Array|Add (Variables|Default|GetR_SocketPositions) (Transformation|GetSocketLocation (Variables|/Script/Engine.SkeletalMeshActor|GetSkeletalMeshComponent (Utilities|Array|Get(acopy) _outactors_2)) "RightWingBase"))
      (for _index_2 (range 1 15)
        (bind _output_get_2 (Variables|Default|SetWingName (Utilities|String|BuildString(Integer) "" "RightWing" _index_2)))
        (Utilities|Array|Add (Variables|Default|GetR_SocketPositions) (Transformation|GetSocketLocation (Variables|/Script/Engine.SkeletalMeshActor|GetSkeletalMeshComponent (Utilities|Array|Get(acopy) _outactors_2)) (Utilities|String|StringToName _output_get_2))))
      (Spline|SetSplinePoints (Variables|Default|GetRightWingSpline) _r_socketpositions "World" true)
      (for _array_element_2 _r_socketpositions
        (bind _returnvalue_2 (AddComponent|AddParticleSystemComponent true (Math|Conversions|ToTransform(Vector) _array_element_2)))
        (Utilities|Array|Add (Variables|Default|GetSpawnedParticles) _returnvalue_2)))))

(event EventTick
  (params (DeltaSeconds :type Float%20%28single-precision%29))
  (bind _rightwingspline (Variables|Default|GetRightWingSpline))
  (bind _leftwingspline (Variables|Default|GetLeftWingSpline))
  (Utilities|FlowControl|Sequence
    (:then_0
      (bind _outactors (Actor|GetAllActorsOfClass "/Game/Eagle/Actors/Eagle_Mesh_Blueprint_Wing.Eagle_Mesh_Blueprint_Wing_C")) ; Update Left Wing Spline and Particle Locations
      (Utilities|Array|Clear (Variables|Default|GetL_SocketPositions))
      (Utilities|Array|Add (Variables|Default|GetL_SocketPositions) (Transformation|GetSocketLocation (Variables|/Script/Engine.SkeletalMeshActor|GetSkeletalMeshComponent (Utilities|Array|Get(acopy) _outactors)) "LeftWingBase"))
      (for _index (range 1 15)
        (bind _output_get (Variables|Default|SetWingName (Utilities|String|BuildString(Integer) "" "LeftWing" _index)))
        (Utilities|Array|Add (Variables|Default|GetL_SocketPositions) (Transformation|GetSocketLocation (Variables|/Script/Engine.SkeletalMeshActor|GetSkeletalMeshComponent (Utilities|Array|Get(acopy) _outactors)) (Utilities|String|StringToName _output_get))))
      (for (_array_element _array_index) (Variables|Default|GetL_SocketPositions)
        (Spline|SetLocationatSplinePoint (Variables|Default|GetLeftWingSpline) _array_index _array_element "World" true))
      (for _index_2 (range 0 (Spline|GetNumberOfSplinePoints _leftwingspline))
        (Transformation|SetWorldLocation (Utilities|Array|Get(acopy) (Variables|Default|GetSpawnedParticles) _index_2) (Spline|GetLocationatSplinePoint _leftwingspline _index_2 "World") false false)))
    (:then_1
      (bind _outactors_2 (Actor|GetAllActorsOfClass "/Game/Eagle/Actors/Eagle_Mesh_Blueprint_Wing.Eagle_Mesh_Blueprint_Wing_C")) ; Update Right Wing Spline and Particle Locations
      (Utilities|Array|Clear (Variables|Default|GetR_SocketPositions))
      (Utilities|Array|Add (Variables|Default|GetR_SocketPositions) (Transformation|GetSocketLocation (Variables|/Script/Engine.SkeletalMeshActor|GetSkeletalMeshComponent (Utilities|Array|Get(acopy) _outactors_2)) "RightWingBase"))
      (for _index_3 (range 1 15)
        (bind _output_get_2 (Variables|Default|SetWingName (Utilities|String|BuildString(Integer) "" "RightWing" _index_3)))
        (Utilities|Array|Add (Variables|Default|GetR_SocketPositions) (Transformation|GetSocketLocation (Variables|/Script/Engine.SkeletalMeshActor|GetSkeletalMeshComponent (Utilities|Array|Get(acopy) _outactors_2)) (Utilities|String|StringToName _output_get_2))))
      (for (_array_element_2 _array_index_2) (Variables|Default|GetR_SocketPositions)
        (Spline|SetLocationatSplinePoint (Variables|Default|GetRightWingSpline) _array_index_2 _array_element_2 "World" true))
      (for _index_4 (range 0 (Spline|GetNumberOfSplinePoints _rightwingspline))
        (Transformation|SetWorldLocation (Utilities|Array|Get(acopy) (Variables|Default|GetSpawnedParticles) (+ _index_4 _array_index_2 0)) (Spline|GetLocationatSplinePoint _rightwingspline _index_4 "World") false false)))))

(fn ConstructionScript)